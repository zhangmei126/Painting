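; BP_Canvas is a paintable canvas actor whose paint coverage comes from a render target.
; The construction script creates a dynamic instance of M_Canvas, applies it to the Cube mesh and sets its PaintColor parameter from a variable.
; On BeginPlay it creates a small render target, clears it to opaque black and binds it as the material's Alpha texture.
; The file itself contains no drawing logic.
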(event EventBeginPlay
  (bind _returnvalue (Rendering|CreateRenderTarget2D 256 256 "RTF_RGBA16f"))
  (bind _output_get (Variables|Default|SetRenderTex _returnvalue))
  (Rendering|ClearRenderTarget2D (Variables|Default|GetRenderTex))
  (Rendering|Material|SetTextureParameterValue (Variables|Default|GetM_Canvas) "Alpha" _output_get))

(fn ConstructionScript
  (bind _returnvalue (Rendering|Material|CreateDynamicMaterialInstance "/Game/Painting/M_Canvas.M_Canvas" "None" :!class /Script/Engine.KismetMaterialLibrary))
  (bind _output_get (Variables|Default|SetM_Canvas _returnvalue))
  (Rendering|Material|SetMaterial (Variables|Default|GetCube) 0 _output_get)
  (Rendering|Material|SetVectorParameterValue (Variables|Default|GetM_Canvas) "PaintColor" (Variables|Default|GetPaintColor) :!class /Script/Engine.MaterialInstanceDynamic))